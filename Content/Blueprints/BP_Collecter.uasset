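; BP_Collecter tracks the fragment collection goal and handles the win.
; On BeginPlay it counts all BP_Fragment actors, then prints the remaining count every tick while the game runs.
; FragmentsRamasse decrements the count and, at zero, triggers Victoire.
; Victory shows a congratulations message, fades the camera to white and, after a delay, opens the Gym_TPFinal level.
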(event Custom|PartieInitialisee
  ;[0.15 0.15 0.15 0.5] Dit que la partie est en cours si il reste des fragments dans la scene
  (Variables|Default|SetPartieEnCours true)
  (bind _outactors (Actor|GetAllActorsOfClass "/Game/Blueprints/BP_Fragment.BP_Fragment_C"))
  (Variables|Default|SetFragmentsRestant (Utilities|Array|Length _outactors)))

(event Custom|FragmentsRamasse
  ;[0.15 0.15 0.15 0.5] Si tous les fragments sont ramasser le joueur gagne
  (bind _result (Math|Integer|DecrementInt (Variables|Default|GetFragmentsRestant))
    (:%20%20
      (Variables|Default|SetFragmentsRestant _result)
      (if (CallFunction|VerifierVictoire)
        (CallFunction|Victoire)))))

(event Custom|Victoire
  ;[0.15 0.15 0.15 0.5] Logique d'affichage de la victoire
  (Variables|Default|SetPartieEnCours false)
  (Development|PrintString "Félicitation !" true true "(R=0.000000,G=1.000000,B=0.201274,A=1.000000)" 4.0)
  (CameraFades|StartCameraFade (Game|GetPlayerCameraManager 0) 0.0 1.0 4.0 "(R=1.000000,G=1.000000,B=1.000000,A=1.000000)" false false)
  (Utilities|FlowControl|Delay 1e+01)
  (Game|OpenLevel(byObjectReference) "/Game/Maps/Gym_TPFinal.Gym_TPFinal"))

(event EventBeginPlay
  (CallFunction|PartieInitialisee))

(event EventTick
  (params (DeltaSeconds :type Float%20%28single-precision%29))
  ;[0.15 0.15 0.15 0.5] Affichage pendant que la partie tourne
  (if (Variables|Default|GetPartieEnCours)
    (Utilities|FlowControl|Sequence
      (:then_1
        (Development|PrintString (Utilities|String|Append "Fragments restants :" (Utilities|String|ToString(Integer) (Variables|Default|GetFragmentsRestant))))))))

(fn ConstructionScript)

(fn VerifierVictoire
  (return (<= (Variables|Default|GetFragmentsRestant) 0)))