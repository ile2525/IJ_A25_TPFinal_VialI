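; BP_Munitions is an ammo pickup that reacts when a BP_FirstPersonCharacter overlaps it.
; On overlap it plays a click sound and destroys itself, before any capacity check, then edits the character's InventaireActuel directly.
; It adds a fixed amount while InventaireActuel is at or below InventaireMax, so the total can exceed the maximum.
; Above the maximum, it subtracts InventaireMax from the current value instead of clamping.
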(event Collision|EventActorBeginOverlap
  (params (OtherActor :type Actor%20Object%20Reference))
  ;[0.15 0.15 0.15 0.5] Joue un son, le détruit et ajoute 10 à l'inventaire si la capacité max n'est pas atteinte
  (bind _asbp_first_person_character (Utilities|Casting|CastToBP_FirstPersonCharacter OtherActor))
  (Audio|PlaySound2D "/Engine/VREditor/Sounds/UI/Click_on_Button.Click_on_Button" 1.0 1.0 0.0 0 0)
  (Actor|DestroyActor)
  (if (<= (Variables|/Game/FirstPerson/Blueprints/BP_FirstPersonCharacter.BP_FirstPersonCharacter_C|GetInventaireActuel _asbp_first_person_character) (Variables|/Game/FirstPerson/Blueprints/BP_FirstPersonCharacter.BP_FirstPersonCharacter_C|GetInventaireMax _asbp_first_person_character))
    (Variables|/Game/FirstPerson/Blueprints/BP_FirstPersonCharacter.BP_FirstPersonCharacter_C|SetInventaireActuel _asbp_first_person_character (+ (Variables|/Game/FirstPerson/Blueprints/BP_FirstPersonCharacter.BP_FirstPersonCharacter_C|GetInventaireActuel _asbp_first_person_character) 1e+01))
    (else
      (Variables|/Game/FirstPerson/Blueprints/BP_FirstPersonCharacter.BP_FirstPersonCharacter_C|SetInventaireActuel _asbp_first_person_character (- (Variables|/Game/FirstPerson/Blueprints/BP_FirstPersonCharacter.BP_FirstPersonCharacter_C|GetInventaireActuel _asbp_first_person_character) (Variables|/Game/FirstPerson/Blueprints/BP_FirstPersonCharacter.BP_FirstPersonCharacter_C|GetInventaireMax _asbp_first_person_character))))))

(fn ConstructionScript)