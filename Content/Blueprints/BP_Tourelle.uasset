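; Turret actor that damages the first-person character on entering its sphere and can be destroyed by point damage.
; Leaving the sphere stores the character as target and re-arms a DoOnce.
; Tick line-traces from the cannon to the target, starting a looping attack timer through the DoOnce on a hit, clearing it otherwise.
; Each attack spawns a projectile at the hit actor's transform, not at the cannon.
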(event OnComponentEndOverlap(Sphere1)
  (params (OverlappedComponent :type Primitive%20Component%20Object%20Reference) (OtherActor :type Actor%20Object%20Reference) (OtherComp :type Primitive%20Component%20Object%20Reference) (OtherBodyIndex :type Integer))
  ;[0.15 0.15 0.15 0.5] Le joueur sort du rayon et n'est plus une cible
  (bind _asbp_first_person_character (Utilities|Casting|CastToBP_FirstPersonCharacter OtherActor))
  (Variables|Default|SetCible _asbp_first_person_character)
  (Rendering|Material|SetMaterial (Variables|Default|GetSphere) 0 "/Game/Materiels/M_Vert.M_Vert")
  (Utilities|Time|ClearandInvalidateTimerbyHandle (Variables|Default|GetAttaqueTimerHandle))
  ;[0.15 0.15 0.15 0.5] Cadence de tir
  (Utilities|FlowControl|DoOnce false) ; enters at Reset
)

(event OnComponentBeginOverlap(Sphere1)
  (params (OverlappedComponent :type Primitive%20Component%20Object%20Reference) (OtherActor :type Actor%20Object%20Reference) (OtherComp :type Primitive%20Component%20Object%20Reference) (OtherBodyIndex :type Integer) (bFromSweep :type Boolean) (SweepResult :type Hit%20Result%20Structure%20%28by%20ref%29))
  ;[0.15 0.15 0.15 0.5] Le joueur entre dans le rayon et devient une cible et prend des degats
  (bind _asbp_first_person_character (Utilities|Casting|CastToBP_FirstPersonCharacter OtherActor))
  (Default|MiseAJourVie _asbp_first_person_character (- (Variables|/Game/FirstPerson/Blueprints/BP_FirstPersonCharacter.BP_FirstPersonCharacter_C|GetPointDeVie _asbp_first_person_character) (Variables|Default|GetDegatsJoueur)))
  (Rendering|Material|SetMaterial (Variables|Default|GetSphere) 0 "/Game/Materiels/M_Vert.M_Vert"))

(event Custom|resetTimer
  ;[0.15 0.15 0.15 0.5] Actualise le timer
  (Utilities|Time|ClearandInvalidateTimerbyHandle (Variables|Default|GetAttaqueTimerHandle)))

(event Custom|CibleDetruite
  ;[0.15 0.15 0.15 0.5] Detruit la cible
  (Actor|DestroyActor))

(event Custom|Attaque
  ;[0.15 0.15 0.15 0.5] Cadence de tir
  (Game|SpawnActorfromClass "/Game/Blueprints/BP_Projectile.BP_Projectile_C" (Transformation|GetActorTransform (.hitactor (stale EventTick _outhit))) "Undefined" "MultiplyWithRoot" 0 0))

(event Game|Damage|EventPointDamage
  (params (Damage :type Float%20%28single-precision%29) (DamageType :type Damage%20Type%20Object%20Reference) (HitLocation :type Vector :default "0, 0, 0") (HitNormal :type Vector :default "0, 0, 0") (HitComponent :type Primitive%20Component%20Object%20Reference) (BoneName :type Name :default "None") (ShotFromDirection :type Vector :default "0, 0, 0") (InstigatedBy :type Controller%20Object%20Reference) (DamageCauser :type Actor%20Object%20Reference) (HitInfo :type Hit%20Result%20Structure%20%28by%20ref%29))
  ;[0.15 0.15 0.15 0.5] Pour appliquer des dégats
  (bind _output_get (Variables|Default|SetNbPointDeVie (- (Variables|Default|GetNbPointDeVie) Damage)))
  (if (<= _output_get 0.0)
    (CallFunction|CibleDetruite)))

(event EventTick
  (params (DeltaSeconds :type Float%20%28single-precision%29))
  (bind _cible (Variables|Default|Getcible))
  (bind _canon (Variables|Default|Getcanon))
  (bind _returnvalue (Transformation|GetWorldLocation _canon))
  ;[0.15 0.15 0.15 0.5] Vérifie si c'est une cible et trace le rayon
  (Utilities|IsValid _cible
    (:Is%20Valid
      (Variables|Default|SetPositionJoueur (- (Transformation|GetActorLocation _cible) (Transformation|GetWorldLocation (Variables|Default|Getcanon))))
      (bind _outhit (Collision|LineTraceByChannel _returnvalue (+ _returnvalue (Variables|Default|GetPositionJoueur)) "TraceTypeQuery2" false 0 "ForOneFrame"))
      ;[0.15 0.15 0.15 0.5] Cadence de tir
      (Utilities|Casting|CastToBP_FirstPersonCharacter (.hitactor _outhit)
        (:then
          (Utilities|FlowControl|DoOnce false
            (:Completed
              (bind _returnvalue_2 (Utilities|Time|SetTimerbyEvent (delegate Custom|Attaque) 1.0 true))
              (Variables|Default|SetAttaqueTimerHandle _returnvalue_2))))
        (:CastFailed
          (CallFunction|ResetTimer))))))

(fn ConstructionScript)